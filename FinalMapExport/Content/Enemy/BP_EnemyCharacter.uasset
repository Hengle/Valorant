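; Enemy character that takes hits by body zone, updates its HP bar and dies.
; HitActor calls ApplyDamage, which walks parent bones looking for Head, then Pelvis, to classify Head, Leg or Body and scale damage.
; Zone picks the sound; zone plus hit direction picks the hit or death montage.
; At zero HP it reports to the player's kill feed, disables collision and destroys itself after a delay.
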(event Custom|HitActor
  (params (Damage :type Float%20%28double-precision%29) (BoneName :type Name) (HitDirection :type Integer) (WeaponIndex :type Enum_WeaponIndex%20Enum :default "NewEnumerator0") (MainWeaponIndex :type Enum_MainWeaponIndex%20Enum :default "NewEnumerator0"))
  (Variables|Default|SetWeapon%20Index WeaponIndex)
  (Variables|Default|SetMain%20Weapon%20Index MainWeaponIndex)
  (CallFunction|ApplyDamage Damage BoneName HitDirection)
  (Audio|PlaySoundatLocation (Utilities|Select :Index (Variables|Default|GetHit%20Bone%20Index) :NewEnumerator0 "/Game/ValorantAsset/Sound/KillSound/Player_Hit/Body/Body_Shot_1_Cue.Body_Shot_1_Cue" :NewEnumerator1 "/Game/ValorantAsset/Sound/KillSound/Player_Hit/Body/Body_Shot_1_Cue.Body_Shot_1_Cue" :NewEnumerator2 "/Game/ValorantAsset/Sound/KillSound/Player_Hit/Headshot/Headshot_1_Cue.Headshot_1_Cue") (Transformation|GetActorLocation) "0, 0, 0" 1.0 1.0 0.0 0 0 0 0)
  (if (<= (Variables|Default|GetHP) 0.0)
    (bind _asbp_first_person_character (Utilities|Casting|CastToBP_FirstPersonCharacter (Game|GetPlayerCharacter 0)))
    (Default|UpdateKillFeed _asbp_first_person_character (Variables|Default|GetEnemyType) (Variables|Default|GetHit%20Bone%20Index) (Variables|Default|GetWeapon%20Index) (Variables|Default|GetMain%20Weapon%20Index))
    (Animation|Montage|PlayMontage (Variables|Character|GetMesh) (Utilities|Array|Get(acopy) (Utilities|Select :Index (Variables|Default|GetHit%20Bone%20Index) :NewEnumerator0 (Variables|Default|GetDeathBody) :NewEnumerator1 (Variables|Default|GetDeathLeg) :NewEnumerator2 (Variables|Default|GetDeathHead)) (Variables|Default|GetHit%20Direction))
      (:then
        (Variables|Default|SetIsDeath true)
        (Collision|SetActorEnableCollision false)
        (Variables|Default|SetAIControllerClass 0)
        (Utilities|FlowControl|Delay 1.2)
        (Actor|DestroyActor)))
    (else
      (Animation|Montage|PlayMontage (Variables|Character|GetMesh) (Utilities|Array|Get(acopy) (Utilities|Select :Index (Variables|Default|GetHit%20Bone%20Index) :NewEnumerator0 (Variables|Default|GetHitBody) :NewEnumerator1 (Variables|Default|GetHitLeg) :NewEnumerator2 (Variables|Default|GetHitHead)) (Variables|Default|GetHit%20Direction))))))

(fn ConstructionScript)

(fn 새함수)

(fn ApplyDamage
  (params (Damage :type Float%20%28double-precision%29) (BoneName :type Name) (HitDirection :type Integer))
  (if (> (Variables|Default|GetHP) 0.0)
    (Variables|Default|SetHit%20Direction HitDirection)
    (Variables|Default|SetDamage Damage)
    (Variables|Default|SetBone%20Name BoneName)
    (bind _isfind (CallFunction|FindParentBone "Head" (Variables|Default|GetBone%20Name)))
    (if _isfind
      (Variables|Default|SetHit%20Bone%20Index "NewEnumerator2")
      (else
        (bind _isfind_2 (CallFunction|FindParentBone "Pelvis" (Variables|Default|GetBone%20Name)))
        (if _isfind_2
          (Variables|Default|SetHit%20Bone%20Index "NewEnumerator1")
          (else
            (Variables|Default|SetHit%20Bone%20Index "NewEnumerator0")))))
    (bind _output_get (Variables|Default|SetHP (- (Variables|Default|GetHP) (* (Variables|Default|GetDamage) (Utilities|Select :Index (Variables|Default|GetHit%20Bone%20Index) :NewEnumerator0 0.8 :NewEnumerator1 0.5 :NewEnumerator2 1.2)))))
    (Progress|SetPercent (.HPBar (Utilities|Struct|BreakST_TopUI (Variables|Default|GetTopUI))) (/ _output_get 1e+02))
    (return)))

(fn FindParentBone
  (params (FindBone :type Name) (StartBone :type Name))
  (LocalVariables|SetCurrentBone StartBone)
  (while (!= (LocalVariables|GetCurrentBone) "Root")
    (if (== (LocalVariables|GetCurrentBone) FindBone)
      (return true)
      (else
        (LocalVariables|SetCurrentBone (Class|SkinnedMeshComponent|GetParentBone (Variables|Character|GetMesh) (LocalVariables|GetCurrentBone))))))
  (return false))

(fn SetAnimation
  (params (AnimArray :type Array%20of%20Anim%20Montage%20Object%20References) (Front :type Anim%20Montage%20Object%20Reference) (Back :type Anim%20Montage%20Object%20Reference) (Right :type Anim%20Montage%20Object%20Reference) (Left :type Anim%20Montage%20Object%20Reference))
  (for _index (range 0 3)
    (Utilities|Array|Add AnimArray (Utilities|Select :Index _index :Option%200 Front :Option%201 Back :Option%202 Right :Option%203 Left))))