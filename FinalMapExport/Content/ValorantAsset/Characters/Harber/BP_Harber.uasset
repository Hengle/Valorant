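; BP_Harber is the Blueprint for the Harber character, supplying its third-person hit-reaction and death montages.
; On BeginPlay, SetAnimation fills separate hit and death arrays for body, head and leg, each with front, back, right and left montages.
; The file has no playback or damage logic, and its construction script only calls the parent's.
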(event EventBeginPlay
  (CallFunction|SetAnimation (Variables|Default|GetHitBody) "/Game/ValorantAsset/Characters/Harber/Animation/Harber_TP_Mage_S0_Skelmesh_TP_Core_HitReact_Body_Front_UB_Montage.Harber_TP_Mage_S0_Skelmesh_TP_Core_HitReact_Body_Front_UB_Montage" "/Game/ValorantAsset/Characters/Harber/Animation/Harber_TP_Mage_S0_Skelmesh_TP_Core_HitReact_Body_Back_UB_Montage.Harber_TP_Mage_S0_Skelmesh_TP_Core_HitReact_Body_Back_UB_Montage" "/Game/ValorantAsset/Characters/Harber/Animation/Harber_TP_Mage_S0_Skelmesh_TP_Core_HitReact_Body_Right_UB_Montage.Harber_TP_Mage_S0_Skelmesh_TP_Core_HitReact_Body_Right_UB_Montage" "/Game/ValorantAsset/Characters/Harber/Animation/Harber_TP_Mage_S0_Skelmesh_TP_Core_HitReact_Body_Left_UB_Montage.Harber_TP_Mage_S0_Skelmesh_TP_Core_HitReact_Body_Left_UB_Montage")
  (CallFunction|SetAnimation (Variables|Default|GetHitLeg) "/Game/ValorantAsset/Characters/Harber/Animation/Harber_TP_Mage_S0_Skelmesh_TP_Core_HitReact_Leg_Front_Montage.Harber_TP_Mage_S0_Skelmesh_TP_Core_HitReact_Leg_Front_Montage" "/Game/ValorantAsset/Characters/Harber/Animation/Harber_TP_Mage_S0_Skelmesh_TP_Core_HitReact_Leg_Back_Montage.Harber_TP_Mage_S0_Skelmesh_TP_Core_HitReact_Leg_Back_Montage" "/Game/ValorantAsset/Characters/Harber/Animation/Harber_TP_Mage_S0_Skelmesh_TP_Core_HitReact_Leg_Right_Montage.Harber_TP_Mage_S0_Skelmesh_TP_Core_HitReact_Leg_Right_Montage" "/Game/ValorantAsset/Characters/Harber/Animation/Harber_TP_Mage_S0_Skelmesh_TP_Core_HitReact_Leg_Left_Montage.Harber_TP_Mage_S0_Skelmesh_TP_Core_HitReact_Leg_Left_Montage")
  (CallFunction|SetAnimation (Variables|Default|GetHitHead) "/Game/ValorantAsset/Characters/Harber/Animation/Harber_TP_Mage_S0_Skelmesh_TP_Core_HitReact_Head_Front_UB_Montage.Harber_TP_Mage_S0_Skelmesh_TP_Core_HitReact_Head_Front_UB_Montage" "/Game/ValorantAsset/Characters/Harber/Animation/Harber_TP_Mage_S0_Skelmesh_TP_Core_HitReact_Head_Back_UB_Montage.Harber_TP_Mage_S0_Skelmesh_TP_Core_HitReact_Head_Back_UB_Montage" "/Game/ValorantAsset/Characters/Harber/Animation/Harber_TP_Mage_S0_Skelmesh_TP_Core_HitReact_Head_Right_UB_Montage.Harber_TP_Mage_S0_Skelmesh_TP_Core_HitReact_Head_Right_UB_Montage" "/Game/ValorantAsset/Characters/Harber/Animation/Harber_TP_Mage_S0_Skelmesh_TP_Core_HitReact_Head_Left_UB_Montage.Harber_TP_Mage_S0_Skelmesh_TP_Core_HitReact_Head_Left_UB_Montage")
  (CallFunction|SetAnimation (Variables|Default|GetDeathBody) "/Game/ValorantAsset/Characters/Harber/Animation/Harber_TP_Mage_S0_Skelmesh_TP_Core_Death_Body_Front_LG_Montage.Harber_TP_Mage_S0_Skelmesh_TP_Core_Death_Body_Front_LG_Montage" "/Game/ValorantAsset/Characters/Harber/Animation/Harber_TP_Mage_S0_Skelmesh_TP_Core_Death_Body_Back_LG_Montage.Harber_TP_Mage_S0_Skelmesh_TP_Core_Death_Body_Back_LG_Montage" "/Game/ValorantAsset/Characters/Harber/Animation/Harber_TP_Mage_S0_Skelmesh_TP_Core_Death_Body_Right_LG_Montage.Harber_TP_Mage_S0_Skelmesh_TP_Core_Death_Body_Right_LG_Montage" "/Game/ValorantAsset/Characters/Harber/Animation/Harber_TP_Mage_S0_Skelmesh_TP_Core_Death_Body_Left_LG_Montage.Harber_TP_Mage_S0_Skelmesh_TP_Core_Death_Body_Left_LG_Montage")
  (CallFunction|SetAnimation (Variables|Default|GetDeathHead) "/Game/ValorantAsset/Characters/Harber/Animation/Harber_TP_Mage_S0_Skelmesh_TP_Core_Death_Head_Front_LG_Montage.Harber_TP_Mage_S0_Skelmesh_TP_Core_Death_Head_Front_LG_Montage" "/Game/ValorantAsset/Characters/Harber/Animation/Harber_TP_Mage_S0_Skelmesh_TP_Core_Death_Head_Back_LG_Montage.Harber_TP_Mage_S0_Skelmesh_TP_Core_Death_Head_Back_LG_Montage" "/Game/ValorantAsset/Characters/Harber/Animation/Harber_TP_Mage_S0_Skelmesh_TP_Core_Death_Head_Right_LG_Montage.Harber_TP_Mage_S0_Skelmesh_TP_Core_Death_Head_Right_LG_Montage" "/Game/ValorantAsset/Characters/Harber/Animation/Harber_TP_Mage_S0_Skelmesh_TP_Core_Death_Head_Left_LG_Montage.Harber_TP_Mage_S0_Skelmesh_TP_Core_Death_Head_Left_LG_Montage")
  (CallFunction|SetAnimation (Variables|Default|GetDeathLeg) "/Game/ValorantAsset/Characters/Harber/Animation/Harber_TP_Mage_S0_Skelmesh_TP_Core_Death_Leg_Front_LG_Montage.Harber_TP_Mage_S0_Skelmesh_TP_Core_Death_Leg_Front_LG_Montage" "/Game/ValorantAsset/Characters/Harber/Animation/Harber_TP_Mage_S0_Skelmesh_TP_Core_Death_Leg_Back_LG_Montage.Harber_TP_Mage_S0_Skelmesh_TP_Core_Death_Leg_Back_LG_Montage" "/Game/ValorantAsset/Characters/Harber/Animation/Harber_TP_Mage_S0_Skelmesh_TP_Core_Death_Leg_Right_LG_Montage.Harber_TP_Mage_S0_Skelmesh_TP_Core_Death_Leg_Right_LG_Montage" "/Game/ValorantAsset/Characters/Harber/Animation/Harber_TP_Mage_S0_Skelmesh_TP_Core_Death_Leg_Left_LG_Montage.Harber_TP_Mage_S0_Skelmesh_TP_Core_Death_Leg_Left_LG_Montage"))

(fn ConstructionScript
  (|CallParentFunction))