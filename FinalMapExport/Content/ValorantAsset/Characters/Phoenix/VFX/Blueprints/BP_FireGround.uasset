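; Phoenix's ground fire area, which burns enemy characters and heals player characters standing inside it.
; Each tick it queries the Sphere's overlaps, calling SkillHit on enemies and Heal on first-person characters, throttled by cooldown flags on those characters.
; A looping one-second timer destroys the actor after roughly ten seconds.
; BeginPlay caches EnemyTeam from the game instance, but this graph never reads it.
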(event Custom|Timer
  (bind _result (Math|Float|IncrementFloat (Variables|Default|GetTime))
    (:%20%20
      (if (> _result 1e+01)
        (Actor|DestroyActor)))))

(event EventTick
  (params (DeltaSeconds :type Float%20%28single-precision%29))
  (for _array_element (Collision|GetOverlappingActors (Variables|Default|GetSphere) "/Game/Enemy/BP_EnemyCharacter.BP_EnemyCharacter_C" :!class /Script/Engine.PrimitiveComponent)
    (Utilities|IsValid _array_element
      (:Is%20Valid
        (bind _asbp_enemy_character (Utilities|Casting|CastToBP_EnemyCharacter _array_element))
        (if (not (Variables|/Game/Enemy/BP_EnemyCharacter.BP_EnemyCharacter_C|GetIsCoolTime _asbp_enemy_character))
          (Default|SkillHit _asbp_enemy_character 3e+01 "NewEnumerator6" "NewEnumerator3")))))
  (for _array_element_2 (Collision|GetOverlappingActors (Variables|Default|GetSphere) "/Game/FirstPerson/Blueprints/BP_FirstPersonCharacter.BP_FirstPersonCharacter_C" :!class /Script/Engine.PrimitiveComponent)
    (Utilities|IsValid _array_element_2
      (:Is%20Valid
        (bind _asbp_first_person_character (Utilities|Casting|CastToBP_FirstPersonCharacter _array_element_2))
        (if (not (Variables|/Game/FirstPerson/Blueprints/BP_FirstPersonCharacter.BP_FirstPersonCharacter_C|GetHealCooltime _asbp_first_person_character))
          (Default|Heal _asbp_first_person_character))))))

(event EventBeginPlay
  (bind _asbp_game_instance (Utilities|Casting|CastToBP_GameInstance (Game|GetGameInstance)))
  (Variables|Default|SetEnemy%20Team (Variables|/Game/BP_GameInstance.BP_GameInstance_C|GetEnemyTeam _asbp_game_instance))
  (Utilities|Time|SetTimerbyEvent (delegate Custom|Timer) 1.0 true))

(fn ConstructionScript)