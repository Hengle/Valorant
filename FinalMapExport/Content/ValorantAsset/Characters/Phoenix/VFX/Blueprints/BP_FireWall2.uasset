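; Phoenix's Blaze fire wall actor, which grows into place when its MakeWall event is called and removes itself afterwards.
; MakeWall plays the cast sound and runs a timeline whose Wall track stretches the actor along X while sliding the Plane component to match.
; When the timeline finishes, it plays the fire loop sound and destroys the actor after a short delay.
; The passed StartLocation is stored but not used in this graph.
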(event Custom|MakeWall
  (params (StartLocation :type Vector))
  (Audio|PlaySoundatLocation "/Game/ValorantAsset/Sound/Phoenix/Skill/Blaze/Blaze_Cast.Blaze_Cast" (Transformation|GetActorLocation) "0, 0, 0" 1.0 1.0 0.0 0 0 0 0)
  (Variables|Default|SetStartLocation StartLocation)
  (bind _wall (Timeline|타임라인 Play)
    (:Update
      (Transformation|SetActorScale3D (Math|Vector|MakeVector (Math|Float|Lerp 0.0 5.0 _wall) 5.0 1.0))
      (Transformation|SetRelativeLocation (Variables|Default|GetPlane) (Math|Vector|MakeVector (* (Math|Float|Lerp 0.0 5.0 _wall) 1e+01) 0.0 2.5e+02) false false))
    (:Finished
      (Audio|PlaySoundatLocation "/Game/ValorantAsset/Sound/Phoenix/Skill/Blaze/Blaze_Fire_Loop_1_Cue.Blaze_Fire_Loop_1_Cue" (Transformation|GetActorLocation) "0, 0, 0" 1.0 1.0 0.0 0 0 0 0)
      (Utilities|FlowControl|Delay 5.0)
      (Actor|DestroyActor))))

(fn ConstructionScript)