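; BP_Bomb is a bomb actor that runs a timed countdown and bursts when it ends.
; On BeginPlay it plays attenuated countdown audio and replaces the timer on player 0's BP_FirstPersonCharacter with one lasting the bomb's Duration.
; After a matching delay it spawns an attached Niagara burst and plays a final sound.
; No damage or destruction logic is present, and nothing runs if the character cast fails.
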(event EventBeginPlay
  (bind _duration (Variables|Default|GetDuration))
  (bind _asbp_first_person_character (Utilities|Casting|CastToBP_FirstPersonCharacter (Game|GetPlayerCharacter 0)))
  (Audio|PlaySoundatLocation "/Game/ValorantAsset/Sound/Weapon/BombCountDownCue.BombCountDownCue" (Transformation|GetActorLocation) "0, 0, 0" 1.0 1.0 0.0 "/Game/ValorantAsset/Sound/Weapon/BombSoundAttenuation.BombSoundAttenuation" "/Game/ValorantAsset/Sound/Weapon/BombSoundConcurrency.BombSoundConcurrency" 0 0)
  (Variables|Default|SetPlayer _asbp_first_person_character)
  (Default|DestoryTimer (Variables|Default|GetPlayer))
  (Default|SetTimer (Variables|Default|GetPlayer) _duration "NewEnumerator2")
  (Utilities|FlowControl|Delay _duration)
  (Niagara|SpawnSystemAttached "/Game/ValorantAsset/Weapons/Bomb/Burst/NS_Burst.NS_Burst" (Variables|Default|GetBomb) "None" "0, 0, 0" "0, 0, 0" "KeepRelativeOffset" true)
  (Audio|PlaySoundatLocation "/Game/ValorantAsset/Sound/Weapon/Bomb/Countdown_3.Countdown_3" (Transformation|GetActorLocation) "0, 0, 0" 1.0 1.0 0.0 "/Game/ValorantAsset/Sound/Weapon/BombSoundAttenuation.BombSoundAttenuation" "/Game/ValorantAsset/Sound/Weapon/BombSoundConcurrency.BombSoundConcurrency" 0 0))

(fn ConstructionScript)