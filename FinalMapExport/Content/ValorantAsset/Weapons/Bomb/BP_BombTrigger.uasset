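; Bomb trigger volume that flags the local player as able to use the bomb and shows the bomb HUD prompt.
; When player pawn 0 enters the Box, it sets IsAbleBomb on BP_FirstPersonCharacter and loops the HUDBomb animation in ping-pong.
; Actor end overlap hides the widget and stops the animation through the begin-overlap cast, but sets IsAbleBomb to true again rather than clearing it.
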(event OnComponentBeginOverlap(Box)
  (params (OverlappedComponent :type Primitive%20Component%20Object%20Reference) (OtherActor :type Actor%20Object%20Reference) (OtherComp :type Primitive%20Component%20Object%20Reference) (OtherBodyIndex :type Integer) (bFromSweep :type Boolean) (SweepResult :type Hit%20Result%20Structure%20%28by%20ref%29))
  (bind _returnvalue (Game|Player|GetPlayerPawn 0))
  (if (== _returnvalue OtherActor)
    (bind _asbp_first_person_character (Utilities|Casting|CastToBP_FirstPersonCharacter _returnvalue))
    (Variables|/Game/FirstPerson/Blueprints/BP_FirstPersonCharacter.BP_FirstPersonCharacter_C|SetIsAbleBomb _asbp_first_person_character true)
    (Widget|SetVisibility (Variables|/Game/ValorantAsset/UI/HUD_1P.HUD_1P_C|GetHUD_Bomb (Variables|/Game/FirstPerson/Blueprints/BP_FirstPersonCharacter.BP_FirstPersonCharacter_C|GetHUD _asbp_first_person_character)) "Visible")
    (UserInterface|Animation|PlayAnimation (Variables|/Game/ValorantAsset/UI/HUD_1P.HUD_1P_C|GetHUD_Bomb (Variables|/Game/FirstPerson/Blueprints/BP_FirstPersonCharacter.BP_FirstPersonCharacter_C|GetHUD _asbp_first_person_character)) (Variables|/Game/ValorantAsset/UI/HUD_Bomb.HUD_Bomb_C|GetAnim_Bomb (Variables|/Game/ValorantAsset/UI/HUD_1P.HUD_1P_C|GetHUD_Bomb (Variables|/Game/FirstPerson/Blueprints/BP_FirstPersonCharacter.BP_FirstPersonCharacter_C|GetHUD _asbp_first_person_character))) 0.0 0 "PingPong" 1.0 false)))

(event Collision|EventActorEndOverlap
  (params (OtherActor :type Actor%20Object%20Reference))
  (bind _returnvalue (Game|Player|GetPlayerPawn 0))
  (if (== _returnvalue OtherActor)
    (bind _asbp_first_person_character (Utilities|Casting|CastToBP_FirstPersonCharacter _returnvalue))
    (Variables|/Game/FirstPerson/Blueprints/BP_FirstPersonCharacter.BP_FirstPersonCharacter_C|SetIsAbleBomb _asbp_first_person_character true)
    (Widget|SetVisibility (Variables|/Game/ValorantAsset/UI/HUD_1P.HUD_1P_C|GetHUD_Bomb (Variables|/Game/FirstPerson/Blueprints/BP_FirstPersonCharacter.BP_FirstPersonCharacter_C|GetHUD (stale OnComponentBeginOverlap(Box) _asbp_first_person_character))) "Hidden")
    (Class|UserWidget|StopAnimation (Variables|/Game/ValorantAsset/UI/HUD_1P.HUD_1P_C|GetHUD_Bomb (Variables|/Game/FirstPerson/Blueprints/BP_FirstPersonCharacter.BP_FirstPersonCharacter_C|GetHUD (stale OnComponentBeginOverlap(Box) _asbp_first_person_character))) (Variables|/Game/ValorantAsset/UI/HUD_Bomb.HUD_Bomb_C|GetAnim_Bomb (Variables|/Game/ValorantAsset/UI/HUD_1P.HUD_1P_C|GetHUD_Bomb (Variables|/Game/FirstPerson/Blueprints/BP_FirstPersonCharacter.BP_FirstPersonCharacter_C|GetHUD (stale OnComponentBeginOverlap(Box) _asbp_first_person_character)))))))

(fn ConstructionScript)