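; BP_EnemyCharacter is an enemy character that takes directional, per-body-part hit damage and plays a matching reaction montage.
; HitActor calls ApplyDamage, which classifies the bone as head, leg or body, prints debug info and subtracts scaled damage from HP.
; The montage comes from per-part arrays indexed by hit direction, with SetAnimation as their fill helper.
; FindParentBone is a stub returning false, so hits currently resolve to body.
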(event Custom|HitActor
  (params (Damage :type Float%20%28double-precision%29) (BoneName :type Name) (HitDirection :type Integer))
  (CallFunction|ApplyDamage Damage BoneName HitDirection)
  (Animation|PlayAnimMontage (Utilities|Array|Get(acopy) (Utilities|Select :Index (Variables|Default|GetHit%20Bone%20Index) :Option%200 (Variables|Default|GetHitBody) :Option%201 (Variables|Default|GetHitLeg) :Option%202 (Variables|Default|GetHitHead)) (Variables|Default|GetHit%20Direction)) 1.0 "None"))

(fn ConstructionScript)

(fn 새함수)

(fn ApplyDamage
  (params (Damage :type Float%20%28double-precision%29) (BoneName :type Name) (HitDirection :type Integer))
  (if (> (Variables|Default|GetHP) 0.0)
    (Variables|Default|SetHit%20Direction HitDirection)
    (Variables|Default|SetDamage Damage)
    (Variables|Default|SetBone%20Name BoneName)
    (bind _isfind (CallFunction|FindParentBone "Head" (Variables|Default|GetBone%20Name)))
    (if _isfind
      (Variables|Default|SetHit%20Bone%20Index 2)
      (else
        (bind _isfind_2 (CallFunction|FindParentBone "Pelvis" (Variables|Default|GetBone%20Name)))
        (if _isfind_2
          (Variables|Default|SetHit%20Bone%20Index 1)
          (else
            (Variables|Default|SetHit%20Bone%20Index 0)))))
    (Utilities|FlowControl|DoOnce false
      (:Completed
        (Development|PrintString (Utilities|Select :Index (Variables|Default|GetHit%20Bone%20Index) :Option%200 "body" :Option%201 "leg" :Option%202 "head"))
        (Development|PrintString (Utilities|Select :Index (Variables|Default|GetHit%20Direction) :Option%200 "front" :Option%201 "back" :Option%202 "right" :Option%203 "left"))
        (Development|PrintString (Utilities|String|ToString(Float) (* (Variables|Default|GetDamage) (Utilities|Select :Index (Variables|Default|GetHit%20Bone%20Index) :Option%200 0.5 :Option%201 0.3 :Option%202 1.0))))
        (Variables|Default|SetHP (- (Variables|Default|GetHP) (* (Variables|Default|GetDamage) (Utilities|Select :Index (Variables|Default|GetHit%20Bone%20Index) :Option%200 0.5 :Option%201 0.3 :Option%202 1.0))))
        (return)))))

(fn FindParentBone
  (params (FindBone :type Name) (StartBone :type Name))
  (return false))

(fn SetAnimation
  (params (AnimArray :type Array%20of%20Anim%20Montage%20Object%20References) (Front :type Anim%20Montage%20Object%20Reference) (Back :type Anim%20Montage%20Object%20Reference) (Right :type Anim%20Montage%20Object%20Reference) (Left :type Anim%20Montage%20Object%20Reference))
  (for _index (range 0 3)
    (Utilities|Array|Add AnimArray (Utilities|Select :Index _index :Option%200 Front :Option%201 Back :Option%202 Right :Option%203 Left))))