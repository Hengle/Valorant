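; Enemy AI controller that runs BT_EnemyBehaviortree on possess and feeds perception results into its Blackboard.
; Sensing an actor tagged Player cancels the forget timer, stores it as EnemyActor and enables the line-of-sight and fire flags.
; Any other perception update disables firing immediately and starts a LineOfSightTimer-length delay before clearing line of sight and target.
; Every perception update also prints a debug "Hello".
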(event OnTargetPerceptionUpdated(AIPerception)
  (params (Actor :type Actor%20Object%20Reference) (Stimulus :type AI%20Stimulus%20Structure))
  (bind _output_get (Variables|Default|SetPlayer Actor))
  (Development|PrintString "Hello")
  (if (and (Actor|ActorHasTag _output_get "Player") (.bSuccessfullySensed (Utilities|Struct|BreakAIStimulus Stimulus)))
    (Utilities|Time|ClearandInvalidateTimerbyHandle (Variables|Default|GetEnemyTimer))
    (AI|Components|Blackboard|SetValueasBool (Variables|Default|GetBlackboard) (Variables|Default|GetHasLineOfSight%20) true)
    (AI|Components|Blackboard|SetValueasObject (Variables|Default|GetBlackboard) (Variables|Default|GetEnemyActor%20) (Variables|Default|GetPlayer))
    (AI|Components|Blackboard|SetValueasBool (Variables|Default|GetBlackboard) (Variables|Default|GetIsAbleFire) true)
    (else
      (AI|Components|Blackboard|SetValueasBool (Variables|Default|GetBlackboard) (Variables|Default|GetIsAbleFire) false)
      (bind _returnvalue (Utilities|Time|SetTimerbyEvent (delegate Custom|StartEnemyTimer) (Variables|Default|GetLineOfSightTimer)))
      (Variables|Default|SetEnemyTimer _returnvalue))))

(event Custom|StartEnemyTimer
  (AI|Components|Blackboard|SetValueasBool (Variables|Default|GetBlackboard) (Variables|Default|GetHasLineOfSight%20) false)
  (AI|Components|Blackboard|SetValueasObject (Variables|Default|GetBlackboard) (Variables|Default|GetEnemyActor%20) 0))

(event EventPossess
  (params (PossessedPawn :type Pawn%20Object%20Reference))
  (AI|RunBehaviorTree "/Game/Enemy/BT_EnemyBehaviortree.BT_EnemyBehaviortree"))

(fn ConstructionScript)