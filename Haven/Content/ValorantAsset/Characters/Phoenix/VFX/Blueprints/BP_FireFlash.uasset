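; Phoenix's fire flash projectile, which flies along a curved path to the left or right of the look direction.
; The Movement event plays a timeline that rebuilds projectile velocity each update, adding a timeline-scaled right vector, negated for left, to the forward look vector.
; The actor destroys itself when the timeline finishes.
; The Hit event is empty, and leftover ground-fire spawn and impulse nodes never run.
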(event Custom|Movement
  (params (IsLeft :type Boolean) (Look :type Vector) (Right :type Vector))
  (bind _projectilemovement (Variables|Default|GetProjectileMovement))
  (Variables|/Script/Engine.ProjectileMovementComponent|SetInitialSpeed _projectilemovement 5e+02)
  (bind _movement (Timeline|타임라인 Play)
    (:Update
      (Variables|/Script/Engine.MovementComponent|SetVelocity _projectilemovement (* (+ (* (Math|Vector|Normalize Right) (Math|Float|SelectFloat (- 0.0 _movement) _movement IsLeft)) (Math|Vector|Normalize Look)) 1e+03)))
    (:Finished
      (Actor|DestroyActor))))

(event Collision|EventHit
  (params (MyComp :type Primitive%20Component%20Object%20Reference) (Other :type Actor%20Object%20Reference) (OtherComp :type Primitive%20Component%20Object%20Reference) (bSelfMoved :type Boolean) (HitLocation :type Vector :default "0, 0, 0") (HitNormal :type Vector :default "0, 0, 0") (NormalImpulse :type Vector :default "0, 0, 0") (Hit :type Hit%20Result%20Structure%20%28by%20ref%29)))

(fn ConstructionScript)