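; Phoenix's fire wall actor, which grows a curved wall steered by the player's facing while it forms.
; MakeWall runs a timeline that extends spline points up to 1000 units along the blend of initial and current forward vectors, using mesh bounds as a spacing threshold.
; Each tick destroys and rebuilds the spline mesh segments between points through Update.
; A ground trace sets StartPoint, which the spline never uses; the construction-script builder is disconnected.
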(event Custom|MakeWall
  (params (PlayerCharacter :type BP%20First%20Person%20Character%20Object%20Reference))
  (bind _splinemeshes (Variables|Default|GetSplineMeshes))
  (bind _returnvalue (AddComponent|AddInstancedStaticMeshComponent false))
  (Variables|Default|SetMinDistance (Math|Vector|VectorLength (- (.Max (Components|StaticMesh|GetLocalBounds _returnvalue)) (.Min (Components|StaticMesh|GetLocalBounds _returnvalue)))))
  (Components|DestroyComponent _returnvalue)
  (Spline|ClearSplinePoints (Variables|Default|GetSpline) true)
  (bind _output_get (Variables|Default|SetPlayer%20Character PlayerCharacter))
  (Variables|Default|SetForward%20Vector (Transformation|GetActorForwardVector _output_get))
  (bind _outhit (Collision|LineTraceByChannel (Transformation|GetActorLocation _output_get) (+ (Transformation|GetActorLocation _output_get) (* (- "" (Math|Vector|Normalize (Transformation|GetActorUpVector _output_get))) 5e+03)) "TraceTypeQuery1" false 0 "None"))
  (Variables|Default|SetStart%20Point (+ (.Location (Collision|BreakHitResult _outhit)) (* (Math|Vector|Normalize (Variables|Default|GetForward%20Vector)) 1e+01)))
  (bind _makewall (Timeline|타임라인 Play)
    (:Update
      (for _array_element _splinemeshes
        (Components|DestroyComponent _array_element))
      (Utilities|Array|Clear _splinemeshes)
      (CallFunction|Update)
      (if (> (Math|Vector|VectorLength (- (Variables|Default|GetPrevPoint) (* (Math|Float|Lerp 0.0 1e+03 _makewall) (Math|Vector|Normalize (+ (Math|Vector|Normalize (Variables|Default|GetForward%20Vector)) (Math|Vector|Normalize (Transformation|GetActorForwardVector (Variables|Default|GetPlayer%20Character)))))))) (Variables|Default|GetMinDistance))
        _
        (else
          (Utilities|FlowControl|DoOnce false
            (:Completed
              _))))
      (Class|SplineComponent|AddPoint (Variables|Default|GetSpline) (Utilities|Struct|MakeSplinePoint (Math|Conversions|ToFloat(Integer) (Spline|GetNumberOfSplinePoints (Variables|Default|GetSpline))) (* (Math|Float|Lerp 0.0 1e+03 _makewall) (Math|Vector|Normalize (+ (Math|Vector|Normalize (Variables|Default|GetForward%20Vector)) (Math|Vector|Normalize (Transformation|GetActorForwardVector (Variables|Default|GetPlayer%20Character)))))) (Math|Vector|MakeVector (.X (Math|Vector|BreakVector (* (Math|Float|Lerp 0.0 1e+03 _makewall) (Math|Vector|Normalize (+ (Math|Vector|Normalize (Variables|Default|GetForward%20Vector)) (Math|Vector|Normalize (Transformation|GetActorForwardVector (Variables|Default|GetPlayer%20Character)))))))) 0.0 0.0) (Math|Vector|MakeVector (.X (Math|Vector|BreakVector (* (Math|Float|Lerp 0.0 1e+03 _makewall) (Math|Vector|Normalize (+ (Math|Vector|Normalize (Variables|Default|GetForward%20Vector)) (Math|Vector|Normalize (Transformation|GetActorForwardVector (Variables|Default|GetPlayer%20Character)))))))) 0.0 0.0) "0.000000,0.000000,0.000000" "1.000000,1.000000,1.000000" "CurveCustomTangent") true)
      (Variables|Default|SetPrevPoint (* (Math|Float|Lerp 0.0 1e+03 _makewall) (Math|Vector|Normalize (+ (Math|Vector|Normalize (Variables|Default|GetForward%20Vector)) (Math|Vector|Normalize (Transformation|GetActorForwardVector (Variables|Default|GetPlayer%20Character))))))))
    (:Finished
      (Class|SplineComponent|AddPoint (Variables|Default|GetSpline) (Utilities|Struct|MakeSplinePoint (Math|Conversions|ToFloat(Integer) (Spline|GetNumberOfSplinePoints (Variables|Default|GetSpline))) (* (Math|Float|Lerp 0.0 1e+03 _makewall) (Math|Vector|Normalize (+ (Math|Vector|Normalize (Variables|Default|GetForward%20Vector)) (Math|Vector|Normalize (Transformation|GetActorForwardVector (Variables|Default|GetPlayer%20Character)))))) (Math|Vector|MakeVector (.X (Math|Vector|BreakVector (* (Math|Float|Lerp 0.0 1e+03 _makewall) (Math|Vector|Normalize (+ (Math|Vector|Normalize (Variables|Default|GetForward%20Vector)) (Math|Vector|Normalize (Transformation|GetActorForwardVector (Variables|Default|GetPlayer%20Character)))))))) 0.0 0.0) (Math|Vector|MakeVector (.X (Math|Vector|BreakVector (* (Math|Float|Lerp 0.0 1e+03 _makewall) (Math|Vector|Normalize (+ (Math|Vector|Normalize (Variables|Default|GetForward%20Vector)) (Math|Vector|Normalize (Transformation|GetActorForwardVector (Variables|Default|GetPlayer%20Character)))))))) 0.0 0.0) "0.000000,0.000000,0.000000" "1.000000,1.000000,1.000000" "CurveCustomTangent") true)
      (CallFunction|Update))))

(event Custom|Update
  (bind _spline (Variables|Default|GetSpline))
  (for _index (range 0 (- (Spline|GetNumberOfSplinePoints (Variables|Default|GetSpline)) 2))
    (bind _returnvalue (AddComponent|AddSplineMeshComponent true))
    (SplineMesh|SetStartandEnd _returnvalue (.Location (Spline|GetLocationandTangentatSplinePoint _spline _index "Local")) (.Tangent (Spline|GetLocationandTangentatSplinePoint _spline _index "Local")) (.Location (Spline|GetLocationandTangentatSplinePoint _spline (+ _index 1) "Local")) (.Tangent (Spline|GetLocationandTangentatSplinePoint _spline (+ _index 1) "Local")) true :!class /Script/Engine.SplineMeshComponent)
    (Transformation|AttachComponentToComponent _returnvalue (Variables|Default|GetDefaultSceneRoot) "None" "KeepRelative" "KeepWorld" "KeepRelative" true)
    (Utilities|Array|Add (Variables|Default|GetSplineMeshes) _returnvalue)))

(fn ConstructionScript)