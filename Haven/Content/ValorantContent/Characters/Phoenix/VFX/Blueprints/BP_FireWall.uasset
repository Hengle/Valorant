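; Phoenix's fire wall actor, which lays a spline along the player's facing from a ground point found by a downward trace.
; MakeWall runs a timeline that adds points out to a fixed length, averaging initial and current forward vectors so turning bends the path.
; On finish, Update loops over the segments but reshapes one shared SplineMesh, leaving it on the last segment.
; Construction-script logic for per-segment meshes is disconnected.
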(event Custom|MakeWall
  (params (PlayerCharacter :type BP%20First%20Person%20Character%20Object%20Reference))
  (Spline|ClearSplinePoints (Variables|Default|GetSpline) true)
  (bind _output_get (Variables|Default|SetPlayer%20Character PlayerCharacter))
  (Variables|Default|SetForward%20Vector (Transformation|GetActorForwardVector _output_get))
  (bind _outhit (Collision|LineTraceByChannel (Transformation|GetActorLocation _output_get) (+ (Transformation|GetActorLocation _output_get) (* (- "" (Math|Vector|Normalize (Transformation|GetActorUpVector _output_get))) 5e+03)) "TraceTypeQuery1" false 0 "None"))
  (Variables|Default|SetStart%20Point (+ (.Location (Collision|BreakHitResult _outhit)) (* (Math|Vector|Normalize (Variables|Default|GetForward%20Vector)) 1e+01)))
  (bind _makewall (Timeline|타임라인 Play)
    (:Update
      (Spline|AddSplinePoint (Variables|Default|GetSpline) (+ (Variables|Default|GetStart%20Point) (* (Math|Float|Lerp 0.0 1e+03 _makewall) (Math|Vector|Normalize (+ (Math|Vector|Normalize (Variables|Default|GetForward%20Vector)) (Math|Vector|Normalize (Transformation|GetActorForwardVector (Variables|Default|GetPlayer%20Character))))))) "World" true)
      (Utilities|FlowControl|DoOnce false))
    (:Finished
      (CallFunction|Update))))

(event Custom|Update
  (bind _spline (Variables|Default|GetSpline))
  (for _index (range 0 (- (Spline|GetNumberOfSplinePoints (Variables|Default|GetSpline)) 2))
    (SplineMesh|SetStartandEnd (Variables|Default|GetSplineMesh) (.Location (Spline|GetLocationandTangentatSplinePoint _spline _index "World")) (.Tangent (Spline|GetLocationandTangentatSplinePoint _spline _index "World")) (.Location (Spline|GetLocationandTangentatSplinePoint _spline (+ _index 1) "World")) (.Tangent (Spline|GetLocationandTangentatSplinePoint _spline (+ _index 1) "World")) true :!class /Script/Engine.SplineMeshComponent)))

(fn ConstructionScript)